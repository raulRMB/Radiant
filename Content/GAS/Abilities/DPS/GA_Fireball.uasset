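; Gameplay ability for a DPS fireball, currently only a debug stub on activation from an event.
; Activation adds replicated loose tags, stores the instigator and prints the target data's hit actor and location, without ending the ability.
; The casting chain is disconnected: it would lock Hero rotation, play a montage and, on its spawn event with authority, commit, spawn a projectile carrying an effect spec, and fire a gameplay cue.
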(event Ability|EventOnEndAbility
  (params (bWasCancelled :type Boolean)))

(event Ability|EventActivateAbilityFromEvent
  (params (EventData :type Gameplay%20Event%20Data%20Structure%20%28by%20ref%29))
  (bind (_eventtag _instigator _target _optionalobject _optionalobject2 _contexthandle _instigatortags _targettags _eventmagnitude _targetdata) (Utilities|Struct|BreakGameplayEventData EventData))
  (bind _returnvalue (Ability|TargetData|GetHitResultfromTargetData _targetdata))
  (Ability|GameplayEffect|AddLooseGameplayTags (Ability|GetOwningActorfromActorInfo) (Variables|Default|GetTag%20Container) true)
  (Variables|Default|SetInstigator _instigator)
  (Development|PrintString (Utilities|GetDisplayName (.hitactor _returnvalue)))
  (Development|PrintString (Utilities|String|ToString(Vector) (.location _returnvalue))))