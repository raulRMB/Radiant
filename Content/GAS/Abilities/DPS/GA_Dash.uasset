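; Dash gameplay ability that teleports the Hero toward the mouse position, capped at MaxRange.
; Non-authority side reads a MouseVec from the event payload, and both paths feed it to a MouseTargetActor for instant target data.
; Valid data locks rotation toward the target, fires start and destination Flash cues and plays the dash montage.
; The montage's notify event commits on authority, teleports without sweep, unlocks rotation and resets movement destination.
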(event Ability|EventOnEndAbility
  (params (bWasCancelled :type Boolean))
  (Class|Hero|SetRotationLock (stale Ability|EventActivateAbilityFromEvent _ashero) false "0, 0, 0"))

(event Ability|EventActivateAbilityFromEvent
  (params (EventData :type Gameplay%20Event%20Data%20Structure%20%28by%20ref%29))
  (bind _returnvalue (Ability|GetAvatarActorfromActorInfo))
  (bind _returnvalue_2 (Ability|GetAvatarActorfromActorInfo))
  (bind _returnvalue_3 (Ability|GetAvatarActorfromActorInfo))
  (bind _returnvalue_4 (Ability|GetAvatarActorfromActorInfo))
  (bind _returnvalue_5 (Transformation|GetActorLocation _returnvalue_2))
  (bind _ashero (Utilities|Casting|CastToHero _returnvalue_3))
  (Class|Hero|SetDestination _ashero (Transformation|GetActorLocation _returnvalue_3))
  (Ability|HasAuthority
    (:True
      _)
    (:False
      (bind _asmouse_vec (Utilities|Casting|CastToMouseVec (.OptionalObject (Utilities|Struct|BreakGameplayEventData EventData))))))
  (bind _data (|WaitTargetData :ConfirmationType "Instant" :Class "/Script/Radiant.MouseTargetActor" :MouseVec (Variables|/Script/Radiant.MouseVec|GetMouseVec _asmouse_vec) :ReticleClass 0)
    (:ValidData
      (bind _returnvalue_6 (Class|Util|GetMouseVecfromTargetData _data))
      (bind _output_get (Variables|Default|SetMousePos _returnvalue_6))
      (bind _ashero_2 (Utilities|Casting|CastToHero _returnvalue_2))
      (Class|Hero|SetRotationLock _ashero_2 true (- _output_get _returnvalue_5))
      (bind _returnvalue_7 (Class|Util|ClampVectorMaxDist (Transformation|GetActorLocation _returnvalue) (Math|Vector|MakeVector (.x (Variables|Default|GetMousePos)) (.y (Variables|Default|GetMousePos)) (.z (Transformation|GetActorLocation _returnvalue))) (Variables|Default|GetMaxRange)))
      (Class|GameplayAbility|ExecuteGameplayCuewithParams "(TagName=\"GameplayCue.Flash\")" (|CollapseGraph_0 _returnvalue_7))
      (Class|GameplayAbility|ExecuteGameplayCuewithParams "(TagName=\"GameplayCue.Flash.Start\")" (|CollapseGraph _returnvalue_5))
      (|PlayMontageandWaitforEvent "None" "/Game/Montages/AM_Dash.AM_Dash" "(GameplayTags=((TagName=\"Ability.Movement.Dash.Notify\")))" 0.05 "None" true 1.0
        (:OnCompleted
          (Ability|EndAbility :!label _label))
        (:OnBlendOut
          (goto _label))
        (:OnInterrupted
          (goto _label))
        (:OnCancelled
          (goto _label))
        (:EventReceived
          (Ability|HasAuthority
            (:True
              (Ability|CommitAbility))
            (:False
              _))
          (bind _returnvalue_8 (Class|Util|ClampVectorMaxDist (Transformation|GetActorLocation _returnvalue_4) (Math|Vector|MakeVector (.x (Variables|Default|GetMousePos)) (.y (Variables|Default|GetMousePos)) (.z (Transformation|GetActorLocation _returnvalue_4))) (Variables|Default|GetMaxRange)))
          (Transformation|SetActorLocation (Ability|GetAvatarActorfromActorInfo) _returnvalue_8 false true)
          (bind _ashero_3 (Utilities|Casting|CastToHero _returnvalue_4))
          (Class|Hero|SetRotationLock _ashero_3 false "0, 0, 0")
          (Class|Hero|ResetDestination _ashero_3))))))