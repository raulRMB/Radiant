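; GA_RangedBasicAttack is a gameplay ability for a hero's ranged basic attack at a selected target.
; It adds replicated loose tags while active and plays the AM_AA montage at increased rate, waiting for the Ability.Spawn.AA event.
; On that event the server spawns BP_TargetedProjectile toward the hero resolved from the stored target ID, carrying a GE_AOE effect spec, then commits and ends.
; The ability also ends when the montage finishes or is interrupted.
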(event Ability|EventActivateAbility
  (bind _returnvalue (Ability|GetAvatarActorfromActorInfo))
  (Ability|GameplayEffect|AddLooseGameplayTags (Ability|GetOwningActorfromActorInfo) (Variables|Default|GetGameplay%20Tags) true)
  (|PlayMontageandWaitforEvent "None" "/Game/Montages/AM_AA.AM_AA" "(GameplayTags=((TagName=\"Ability.Spawn.AA\")))" 4.0 "None" false 1.0
    (:OnCompleted
      (Ability|EndAbility :!label _label))
    (:OnBlendOut
      (goto _label))
    (:OnInterrupted
      (goto _label))
    (:OnCancelled
      (goto _label))
    (:EventReceived
      (Ability|HasAuthority
        (:True
          (bind _ashero (Utilities|Casting|CastToHero _returnvalue))
          (bind _returnvalue_2 (Class|Util|GetHerofromPlayerID _ashero (Class|Hero|GetTargetID _ashero)))
          (Game|SpawnActorfromClass "/Game/Blueprints/Combat/BP_TargetedProjectile.BP_TargetedProjectile_C" (Transformation|GetActorTransform _ashero) "Undefined" 0 (Ability|MakeOutgoingGameplayEffectSpec "/Game/GAS/Effects/AOE/GE_AOE.GE_AOE_C") _returnvalue_2 (.AsPawn (Utilities|Casting|CastToPawn _returnvalue)))
          (Ability|CommitAbility)
          (Ability|EndAbility))))))

(event Ability|EventOnEndAbility
  (params (bWasCancelled :type Boolean))
  (Ability|GameplayEffect|RemoveLooseGameplayTags (Ability|GetOwningActorfromActorInfo) (Variables|Default|GetGameplay%20Tags) true))