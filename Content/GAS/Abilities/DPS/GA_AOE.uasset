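; GA_AOE is a DPS gameplay ability that launches a Void Implosion projectile toward the player's mouse position.
; Instant target data from MouseTargetActor supplies the point, with non-authority instances feeding in the MouseVec from the activation event.
; The Hero locks rotation toward it during the montage, whose gameplay event makes the server commit and spawn BP_Projectile_Child with range and effect specs.
; That event also clears the loose tags and rotation lock.
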(event Ability|EventActivateAbilityFromEvent
  (params (EventData :type Gameplay%20Event%20Data%20Structure%20%28by%20ref%29))
  (bind _returnvalue (Ability|GetAvatarActorfromActorInfo))
  (bind _returnvalue_2 (Ability|GetAvatarActorfromActorInfo))
  (bind _gameplay_effect_class (Variables|Default|GetGameplay%20Effect%20Class))
  (bind _returnvalue_3 (Transformation|GetActorLocation _returnvalue_2))
  (bind _returnvalue_4 (Ability|MakeOutgoingGameplayEffectSpec _gameplay_effect_class))
  (Ability|GameplayEffect|AddLooseGameplayTags (Ability|GetOwningActorfromActorInfo) (Variables|Default|GetGameplay%20Tags) true)
  (Ability|HasAuthority
    (:True
      _)
    (:False
      (bind _asmouse_vec (Utilities|Casting|CastToMouseVec (.OptionalObject (Utilities|Struct|BreakGameplayEventData EventData))))))
  (bind _data (|WaitTargetData :ConfirmationType "Instant" :Class "/Script/Radiant.MouseTargetActor" :MouseVec (Variables|/Script/Radiant.MouseVec|GetMouseVec _asmouse_vec) :ReticleClass 0)
    (:ValidData
      (bind _returnvalue_5 (Class|Util|GetMouseVecfromTargetData _data))
      (bind _output_get (Variables|Default|SetMousePos _returnvalue_5))
      (bind _ashero (Utilities|Casting|CastToHero _returnvalue))
      (Class|Hero|SetRotationLock _ashero true (- _output_get (Transformation|GetActorLocation _returnvalue)))
      (|PlayMontageandWaitforEvent "None" "/Game/Montages/AM_VoidImplostion.AM_VoidImplostion" "(GameplayTags=((TagName=\"Ability.Combat.AOE.VoidImplosion\")))" 3.0 "None" true 1.0
        (:OnCompleted
          (Ability|EndAbility :!label _label))
        (:OnBlendOut
          (goto _label))
        (:OnInterrupted
          (goto _label))
        (:OnCancelled
          (goto _label))
        (:EventReceived
          (Ability|HasAuthority
            (:True
              (Ability|CommitAbility)
              (Game|SpawnActorfromClass "/Game/Blueprints/Combat/BP_Projectile_Child.BP_Projectile_Child_C" (Math|Transform|MakeTransform (+ _returnvalue_3 (* (Transformation|GetActorForwardVector _returnvalue_2) (Variables|Default|GetForwardDist))) (Transformation|GetActorRotation _returnvalue_2)) "Undefined" 0 (- (Math|Vector|Distance(Vector) (Variables|Default|GetMousePos) _returnvalue_3) (Variables|Default|GetForwardDist)) _returnvalue_4 _returnvalue_4 (.AsPawn (Utilities|Casting|CastToPawn (Ability|GetAvatarActorfromActorInfo)))))
            (:False
              _))
          (bind _ashero_2 (Utilities|Casting|CastToHero (Ability|GetAvatarActorfromActorInfo)))
          (Class|Hero|SetRotationLock _ashero_2 false "0, 0, 0")
          (Ability|GameplayEffect|RemoveLooseGameplayTags (Ability|GetOwningActorfromActorInfo) (Variables|Default|GetGameplay%20Tags) true))))))

(event Ability|EventOnEndAbility
  (params (bWasCancelled :type Boolean))
  (bind _ashero (Utilities|Casting|CastToHero (Ability|GetAvatarActorfromActorInfo)))
  (Class|Hero|SetRotationLock _ashero false "0, 0, 0"))