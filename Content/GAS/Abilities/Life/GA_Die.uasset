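; GA_Die is the Gameplay Ability that handles a BP_Ninja character's death.
; On activation it adds replicated loose tags, applies GE_Death, fires the death cue and starts AM_Death.
; As the montage starts, it applies the respawn timer effect and the server calls SetCollision on the ninja.
; The montage's States.Dead event makes the server hide the ninja, then the ability ends on server and client.
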(event Ability|EventActivateAbility
  (Ability|GameplayEffect|AddLooseGameplayTags (Ability|GetOwningActorfromActorInfo) (Variables|Default|GetGameplay%20Tags) true)
  (Ability|ApplyGameplayEffectSpecToOwner (Ability|MakeOutgoingGameplayEffectSpec "/Game/GAS/Effects/Life/GE_Death.GE_Death_C"))
  (GameplayCue|ExecuteGameplayCue :GameplayCueTag "(TagName=\"GameplayCue.Life.Die\")")
  (|PlayMontageandWaitforEvent "None" "/Game/Characters/Avatars/DPS/NinjaAssets/Montages/AM_Death.AM_Death" "(GameplayTags=((TagName=\"States.Dead\")))" 1.0 "None" true 1.0
    (:then
      (Ability|ApplyGameplayEffectToOwner "/Game/GAS/Effects/Life/GE_SetRespawnTimer.GE_SetRespawnTimer_C")
      (Ability|HasAuthority
        (:True
          (bind _asbp_ninja (Utilities|Casting|CastToBP_Ninja (Ability|GetAvatarActorfromActorInfo)))
          (Default|SetCollision _asbp_ninja _asbp_ninja))))
    (:EventReceived
      (Ability|HasAuthority
        (:True
          (bind _asbp_ninja_2 (Utilities|Casting|CastToBP_Ninja (Ability|GetAvatarActorfromActorInfo)))
          (Default|SetVisiblity _asbp_ninja_2 false _asbp_ninja_2))
        (:False
          _))
      (Ability|EndAbility))))

(event Ability|EventOnEndAbility
  (params (bWasCancelled :type Boolean)))