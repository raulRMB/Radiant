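; Child projectile that bursts into a BP_AOE area-of-effect actor when it overlaps something or ends its flight.
; It records its start position on BeginPlay and checks travelled distance against MaxDist every tick.
; Sphere overlap, reaching MaxDist or OnLifeOver each make the server alone spawn the AOE at the projectile's transform and destroy the projectile.
; The AOE receives the projectile's spec handle and instigator.
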(event OnComponentBeginOverlap(Sphere)
  (params (OverlappedComponent :type Primitive%20Component%20Object%20Reference) (OtherActor :type Actor%20Object%20Reference) (OtherComp :type Primitive%20Component%20Object%20Reference) (OtherBodyIndex :type Integer) (bFromSweep :type Boolean) (SweepResult :type Hit%20Result%20Structure%20%28by%20ref%29))
  (bind _returnvalue (Transformation|GetActorTransform))
  (Networking|SwitchHasAuthority
    (:Authority
      (Game|SpawnActorfromClass "/Game/Combat/BP_AOE.BP_AOE_C" (Math|Transform|MakeTransform (Math|Vector|MakeVector (.x (.location _returnvalue)) (.y (.location _returnvalue)) (.z (.location _returnvalue))) (.rotation _returnvalue) (.scale _returnvalue)) "Undefined" 0 (Variables|Default|GetSpec%20Handle_0) (Game|GetInstigator))
      (Actor|DestroyActor))))

(event EventBeginPlay
  (|CallParentFunction)
  (Variables|Default|SetStartPos (Transformation|GetActorLocation)))

(event Collision|EventActorBeginOverlap
  (params (OtherActor :type Actor%20Object%20Reference)))

(event EventTick
  (params (DeltaSeconds :type Float%20%28single-precision%29))
  (bind _returnvalue (Transformation|GetActorTransform))
  (Variables|Default|SetTravelDist (Math|Vector|Distance(Vector) (Variables|Default|GetStartPos) (Transformation|GetActorLocation)))
  (if (>= (Variables|Default|GetTravelDist) (Variables|Default|GetMaxDist))
    (Networking|SwitchHasAuthority
      (:Authority
        (Game|SpawnActorfromClass "/Game/Combat/BP_AOE.BP_AOE_C" (Math|Transform|MakeTransform (Math|Vector|MakeVector (.x (.location _returnvalue)) (.y (.location _returnvalue)) (.z (.location _returnvalue))) (.rotation _returnvalue) (.scale _returnvalue)) "Undefined" 0 (Variables|Default|GetSpec%20Handle_0) (Game|GetInstigator))
        (Actor|DestroyActor)))))

(event EventOnLifeOver
  (bind _returnvalue (Transformation|GetActorTransform))
  (Networking|SwitchHasAuthority
    (:Authority
      (Game|SpawnActorfromClass "/Game/Combat/BP_AOE.BP_AOE_C" (Math|Transform|MakeTransform (Math|Vector|MakeVector (.x (.location _returnvalue)) (.y (.location _returnvalue)) (.z (.location _returnvalue))) (.rotation _returnvalue) (.scale _returnvalue)) "Undefined" 0 (Variables|Default|GetSpec%20Handle_0) (Game|GetInstigator))
      (Actor|DestroyActor))))

(fn ConstructionScript
  (|CallParentFunction))