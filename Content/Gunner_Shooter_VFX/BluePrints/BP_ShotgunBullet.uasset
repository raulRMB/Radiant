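; BP_ShotgunBullet is a short-lived shotgun projectile actor with a Niagara effect and a capsule for hit detection.
; On BeginPlay it times out after a brief delay, deactivating the effect, destroying the capsule, then destroying itself.
; A capsule overlap with an Enemy- or Obstacle-tagged actor spawns the impact Niagara system at that actor's location, then deactivates the trail and destroys the bullet after a short delay.
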(event OnComponentBeginOverlap(Capsule1)
  (params (OverlappedComponent :type Primitive%20Component%20Object%20Reference) (OtherActor :type Actor%20Object%20Reference) (OtherComp :type Primitive%20Component%20Object%20Reference) (OtherBodyIndex :type Integer) (bFromSweep :type Boolean) (SweepResult :type Hit%20Result%20Structure%20%28by%20ref%29))
  (if (or (Actor|ActorHasTag OtherActor "Enemy") (Actor|ActorHasTag OtherActor "Obstacle"))
    (Niagara|SpawnSystematLocation "/Game/Gunner_Shooter_VFX/Effects/ShotgunShot/NS_Shotgun_Impact.NS_Shotgun_Impact" (Transformation|GetActorLocation OtherActor))
    (Components|Activation|Deactivate (Variables|Default|GetNiagara))
    (Utilities|FlowControl|Delay 0.2)
    (Actor|DestroyActor)))

(event EventBeginPlay
  (Utilities|FlowControl|Delay 0.18)
  (Components|Activation|Deactivate (Variables|Default|GetNiagara))
  (Components|DestroyComponent (Variables|Default|GetCapsule1))
  (Utilities|FlowControl|Delay 0.2)
  (Actor|DestroyActor))

(event Collision|EventActorBeginOverlap
  (params (OtherActor :type Actor%20Object%20Reference)))

(event EventTick
  (params (DeltaSeconds :type Float%20%28single-precision%29)))

(fn ConstructionScript)