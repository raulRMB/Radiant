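; Falling end stage of the Gunner area shot bullet, which drops a Niagara effect and spawns an area explosion below.
; On BeginPlay it moves the Niagara component downward over a short time, then sweeps the capsule down by the same distance.
; The sweep hit location places the explosion system, and the falling effect deactivates after a brief delay.
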(event EventBeginPlay
  (Components|MoveComponentTo (Variables|Default|GetNiagara) "0.000000,0.000000,-1500.000000" "0, 0, 0" false false 0.5 false)
  (bind _sweephitresult (Transformation|SetWorldLocation (Variables|Default|GetCapsule) (+ (Transformation|GetActorLocation) "0, 0,-1500.000000") true false))
  (Niagara|SpawnSystematLocation "/Game/Gunner_Shooter_VFX/Effects/AreaShot/NS_AreaShot_Area_Explosion.NS_AreaShot_Area_Explosion" (.Location (Collision|BreakHitResult _sweephitresult)))
  (Utilities|FlowControl|Delay 0.2)
  (Components|Activation|Deactivate (Variables|Default|GetNiagara)))

(fn ConstructionScript)