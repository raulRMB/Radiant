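; A basic-shot bullet Blueprint from a gunner shooter VFX set that reacts to hitting actors tagged Enemy or Obstacle.
; Capsule overlap deactivates the bullet's Niagara effect, then destroys the actor after a short delay.
; An impact Niagara system also spawns at the hit actor's location, facing the bullet's forward vector, unless HasCollided is true.
; The graph reads HasCollided but never sets it.
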(event OnComponentBeginOverlap(Capsule1)
  (params (OverlappedComponent :type Primitive%20Component%20Object%20Reference) (OtherActor :type Actor%20Object%20Reference) (OtherComp :type Primitive%20Component%20Object%20Reference) (OtherBodyIndex :type Integer) (bFromSweep :type Boolean) (SweepResult :type Hit%20Result%20Structure%20%28by%20ref%29))
  (bind _returnvalue (Actor|ActorHasTag OtherActor "Obstacle"))
  (bind _returnvalue_2 (Actor|ActorHasTag OtherActor "Enemy"))
  (bind _returnvalue_3 (or _returnvalue_2 _returnvalue))
  (if (Variables|Default|GetHas%20collided)
    (if _returnvalue_3
      (Components|Activation|Deactivate (Variables|Default|GetNiagara))
      (Utilities|FlowControl|Delay 1.0)
      (Actor|DestroyActor))
    (elif _returnvalue_3
      (Niagara|SpawnSystematLocation "/Game/Gunner_Shooter_VFX/Effects/BasicShot_2/NS_BasicShot_2_Impact.NS_BasicShot_2_Impact" (Transformation|GetActorLocation OtherActor) (Math|Conversions|RotationFromXVector (Transformation|GetActorForwardVector)))
      (Components|Activation|Deactivate (Variables|Default|GetNiagara))
      (Utilities|FlowControl|Delay 1.0)
      (Actor|DestroyActor))))

(event EventBeginPlay)

(event Collision|EventActorBeginOverlap
  (params (OtherActor :type Actor%20Object%20Reference)))

(event EventTick
  (params (DeltaSeconds :type Float%20%28single-precision%29)))

(fn ConstructionScript)