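; BP_AOE is a combat area-of-effect actor that applies a gameplay effect to heroes near where it spawns.
; On BeginPlay it runs a single sphere overlap at its location, filtered to BP_Hero and ignoring its instigator.
; For each hit that passes a cast, the ability system component on that hero's PlayerState applies the stored effect spec to itself.
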(event EventBeginPlay
  (bind _outactors (Collision|SphereOverlapActors (Transformation|GetActorLocation) 5e+02 (Variables|Default|GetObject%20Types) "/Game/Blueprints/BP_Hero.BP_Hero_C" (Utilities|Array|MakeArray (Game|GetInstigator))))
  (for _array_element _outactors
    (bind _ashero (Utilities|Casting|CastTo _array_element))
    (GameplayEffects|ApplyGameplayEffectSpecToTarget (Ability|GetAbilitySystemComponent (Variables|/Script/Engine.Pawn|GetPlayerState _ashero)) (Variables|Default|GetSpec%20Handle) (Ability|GetAbilitySystemComponent (Variables|/Script/Engine.Pawn|GetPlayerState _ashero)))))

(fn ConstructionScript)