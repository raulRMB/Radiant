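; BP_Projectile is a short-lived combat projectile that delivers a gameplay effect to the character it hits.
; It destroys itself after a brief delay from BeginPlay.
; On sphere overlap it skips its instigator, finds the Ability System Component on the hit character's PlayerState, and has that component apply the stored effect spec to itself.
; The projectile is destroyed on that hit; targets without a valid component leave it alive.
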(event OnComponentBeginOverlap(Sphere)
  (params (OverlappedComponent :type Primitive%20Component%20Object%20Reference) (OtherActor :type Actor%20Object%20Reference) (OtherComp :type Primitive%20Component%20Object%20Reference) (OtherBodyIndex :type Integer) (bFromSweep :type Boolean) (SweepResult :type Hit%20Result%20Structure%20%28by%20ref%29))
  (if (!= OtherActor (Game|GetInstigator))
    (bind _ascharacter (Utilities|Casting|CastToCharacter OtherActor))
    (Utilities|IsValid (Ability|GetAbilitySystemComponent (Variables|/Script/Engine.Pawn|GetPlayerState _ascharacter))
      (:Is%20Valid
        (GameplayEffects|ApplyGameplayEffectSpecToTarget (Ability|GetAbilitySystemComponent (Variables|/Script/Engine.Pawn|GetPlayerState _ascharacter)) (Variables|Default|GetSpec%20Handle) (Ability|GetAbilitySystemComponent (Variables|/Script/Engine.Pawn|GetPlayerState _ascharacter)))
        (Actor|DestroyActor)))))

(event Custom|OnLifeOver
  (Actor|DestroyActor))

(event EventBeginPlay
  (Utilities|FlowControl|Delay 0.8)
  (CallFunction|OnLifeOver))

(fn ConstructionScript)